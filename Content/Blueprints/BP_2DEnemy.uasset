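; BP_2DEnemy is a 2D flipbook-animated enemy character with movement animations and landing effects.
; Tick picks jump, run or idle flipbooks from the Alive and Jumping flags and velocity, printing debug text for run and idle.
; OnLanded spawns an impact particle and sound at the feet, then disables input for the sprite's flipbook length before clearing Jumping.
; PlayNewFlipbook is an empty stub, and the not-Alive branch passes it no flipbook.
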(event EventTick
  (params (DeltaSeconds :type Float%20%28single-precision%29))
  (bind _self self)
  (bind _returnvalue (Transformation|GetVelocity _self))
  (bind (_x _y _z) (Math|Vector|BreakVector _returnvalue))
  ;[0.1485 0.15 0 0.5] Animation and Effects Handlers
  (if (Variables|Default|GetAlive)
    (if (Variables|Default|GetJumping)
      (if (> _z 0.0)
        ;;[1 0.501 0 0.5] Animations
        (CallFunction|PlayNewFlipbook false "/Game/Flipbooks/SOURCE/FB_JumpStart.FB_JumpStart")
        (Variables|Default|SetJumping true)
        (elif (< _z 0.0)
          (CallFunction|PlayNewFlipbook false "/Game/Flipbooks/SOURCE/FB_JumpDown.FB_JumpDown")
          (Variables|Default|SetJumping true)))
      (elif (or (> _x 0.0) (< _x 0.0))
        (CallFunction|PlayNewFlipbook true "/Game/Flipbooks/SOURCE/FASTRUN.FASTRUN")
        (Development|PrintString "run")
        (elif (== _x 0.0)
          (CallFunction|PlayNewFlipbook false "/Game/Flipbooks/SOURCE/IDLE.IDLE")
          (Development|PrintString "idle"))))
    (else
      (CallFunction|PlayNewFlipbook false)
      (Utilities|FlowControl|Delay (Class|PaperFlipbookComponent|GetFlipbookLength (Variables|Default|GetSprite))))))

(event EventOnLanded
  (params (Hit :type Hit%20Result%20Structure%20%28by%20ref%29))
  (bind _location (Collision|BreakHitResult Hit))
  (bind _capsulecomponent (Variables|Collision|GetCapsuleComponent))
  (bind _capsulehalfheight (Variables|/Script/Engine.CapsuleComponent|GetCapsuleHalfHeight _capsulecomponent))
  (bind _returnvalue (- _location (Math|Vector|MakeVector 0.0 0.0 _capsulehalfheight)))
  ;[0.1485 0.15 0 0.5] Animation and Effects Handlers
  ;;[1 1 1] Landing Effects and Animations
  (Effects|SpawnEmitteratLocation "/Game/ImportedContent/InfinityBladeEffects/Effects/FX_Cines/Ausar/P_CIN_Ausar_Player_Impact.P_CIN_Ausar_Player_Impact" _returnvalue)
  (Audio|PlaySoundatLocation "/Game/Sounds/SFX/269781-gritty-concrete-trainers-landing-nt1a_f6XGDvfS.269781-gritty-concrete-trainers-landing-nt1a_f6XGDvfS" _returnvalue "0, 0, 0" 1.0 1.0 0.0 0 0 0 0)
  ;;;[1 0.501 0 0.5] Animations
  (CallFunction|PlayNewFlipbook false "/Game/Flipbooks/SOURCE/FB_JumpLand.FB_JumpLand")
  (Input|DisableInput 0)
  (Utilities|FlowControl|Delay (Class|PaperFlipbookComponent|GetFlipbookLength (Variables|Default|GetSprite)))
  (Input|EnableInput 0)
  (Variables|Default|SetJumping false))

(fn ConstructionScript)

(fn PlayNewFlipbook
  (params (bNewLooping :type Boolean) (NewFlipbook :type Paper%20Flipbook%20Object%20Reference)))